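; BP_Weapon is a weapon Blueprint with a debug-stage hitscan test bound directly to the 1 key.
; On press, it line-traces on the Camera channel from its owner's location along the owner's forward vector for GunRange, ignoring the owner's child actors.
; The trace is drawn for a duration and the hit actor's name is printed, with no damage or effects applied.
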(event `Key|One`
  (params (Key :type "Key Structure"))
  (bind _returnvalue (`self.GetOwner`))
  (bind _returnvalue_2 (`Actor.K2_GetActorLocation` _returnvalue))
  (:`Pressed`
    (bind _outhit (`KismetSystemLibrary.LineTraceSingle` _returnvalue_2 (+ (* (`Actor.GetActorForwardVector` _returnvalue) (`self.GunRange`)) _returnvalue_2) "TraceTypeQuery2" false (`Actor.GetAllChildActors` _returnvalue true) "ForDuration"))
    (`KismetSystemLibrary.PrintString` (`KismetSystemLibrary.GetDisplayName` (`.HitActor` (`GameplayStatics.BreakHitResult` _outhit))))))